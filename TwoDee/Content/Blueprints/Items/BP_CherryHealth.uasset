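; BP_CherryHealth is a cherry pickup that restores one point of health to the player character.
; A box overlap with BP_PlayerChar calls ChangeHealth, swaps the flipbook to a feedback animation and reveals the HPText widget component.
; That component's WB_HPGain widget plays its gain display, and the actor destroys itself after a short delay.
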(event OnComponentBeginOverlap(Box)
  (params (OverlappedComponent :type Primitive%20Component%20Object%20Reference) (OtherActor :type Actor%20Object%20Reference) (OtherComp :type Primitive%20Component%20Object%20Reference) (OtherBodyIndex :type Integer) (bFromSweep :type Boolean) (SweepResult :type Hit%20Result%20Structure%20%28by%20ref%29))
  (bind _hptext (Variables|Default|GetHPText))
  (bind _asbp_player_char (Utilities|Casting|CastToBP_PlayerChar OtherActor))
  (Default|ChangeHealth _asbp_player_char 1)
  (Sprite|SetFlipbook (Variables|Default|GetRenderComponent) "/Game/SunnyLandAssets/sprites/item-feedback/item-feedback.item-feedback")
  (Development|SetHiddeninGame _hptext false false)
  (bind _aswb_hpgain (Utilities|Casting|CastToWB_HPGain (UserInterface|GetUserWidgetObject _hptext)))
  (Default|ShowHPGain _aswb_hpgain)
  (Utilities|FlowControl|Delay 0.8)
  (Actor|DestroyActor))

(fn ConstructionScript)