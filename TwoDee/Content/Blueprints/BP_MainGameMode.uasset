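; Game mode that runs the room-to-room transition sequence when the player passes through a door.
; RoomTransition hides the player and fades sprites to black via an Opacity parameter in a material parameter collection driven by timelines.
; It then teleports the player to their stored spawn location, blends the view to their current room camera, fades back in and clears the door-movement flag to restore control.
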(event Custom|RoomTransition
  ;[0 0 0] Room transition sequence when player enters a Door
  (bind _asbp_player_char (Utilities|Casting|CastToBP_PlayerChar (Game|Player|GetPlayerPawn 0)))
  ;;[0 0 0] Hides player character
  (Rendering|SetActorHiddenInGame _asbp_player_char true)
  ;;[0 0 0] Sprites with TransitionSpriteMaterial fade to black
  (bind _opacity (Timeline|SpriteFadeoutTimeline PlayFromStart)
    (:Update
      (Rendering|Material|SetScalarParameterValue "/Game/Materials/TransitionParamCollection.TransitionParamCollection" "Opacity" (Math|Float|Lerp 0.0 1.0 _opacity) :!class /Script/Engine.KismetMaterialLibrary))
    (:OnComplete
      ;;[0 0 0] Teleports player to other side of door and un-hides them
      (Transformation|Teleport _asbp_player_char (Variables|/Game/Blueprints/Player/BP_PlayerChar.BP_PlayerChar_C|GetNewSpawnLocation _asbp_player_char) "0, 0, 0")
      (Rendering|SetActorHiddenInGame _asbp_player_char false)
      ;;[0 0 0] Transitions camera to next room
      (Game|Player|SetViewTargetwithBlend (Game|GetPlayerController 0) (Variables|/Game/Blueprints/Player/BP_PlayerChar.BP_PlayerChar_C|GetCurrentCam _asbp_player_char) 0.75 "VTBlend_EaseInOut" 2.0 false)
      (Utilities|FlowControl|Delay 0.75)
      ;;[0 0 0] Sprites fade from black to normal color
      (bind _opacity_2 (Timeline|SpriteFadeinTimeline PlayFromStart)
        (:Update
          (Rendering|Material|SetScalarParameterValue "/Game/Materials/TransitionParamCollection.TransitionParamCollection" "Opacity" (Math|Float|Lerp 1.0 0.0 _opacity_2) :!class /Script/Engine.KismetMaterialLibrary))
        (:OnComplete
          ;;[0 0 0] Re-enables player control over movement
          (Variables|/Game/Blueprints/Player/BP_PlayerChar.BP_PlayerChar_C|SetIsMovingThroughDoor _asbp_player_char false))))))

(fn ConstructionScript)