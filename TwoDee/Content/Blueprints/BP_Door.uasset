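; BP_Door links two rooms, sending the player to the opposite side when they walk into either of its triggers.
; On BeginPlay, after a zero Delay, it caches the BP_Camera overlapping each side's spawn location.
; A trigger overlap flags BP_PlayerChar as moving through a door and sets its new spawn point and camera to the far side.
; It then calls RoomTransition on BP_MainGameMode.
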(event OnComponentBeginOverlap(DoorTriggerRight)
  (params (OverlappedComponent :type Primitive%20Component%20Object%20Reference) (OtherActor :type Actor%20Object%20Reference) (OtherComp :type Primitive%20Component%20Object%20Reference) (OtherBodyIndex :type Integer) (bFromSweep :type Boolean) (SweepResult :type Hit%20Result%20Structure%20%28by%20ref%29))
  ;[0 0 0] Door transition triggers
  (bind _asbp_player_char (Utilities|Casting|CastToBP_PlayerChar OtherActor))
  (Variables|/Game/Blueprints/BP_PlayerChar.BP_PlayerChar_C|SetIsMovingThroughDoor _asbp_player_char true)
  (Variables|/Game/Blueprints/BP_PlayerChar.BP_PlayerChar_C|SetNewSpawnLocation _asbp_player_char (Transformation|GetWorldLocation (Variables|Default|GetLeftSpawnLocation)))
  (Variables|/Game/Blueprints/BP_PlayerChar.BP_PlayerChar_C|SetCurrentCam _asbp_player_char (Variables|Default|GetLeftCamera))
  (bind _asbp_main_game_mode (Utilities|Casting|CastToBP_MainGameMode (Game|GetGameMode)))
  (Default|RoomTransition _asbp_main_game_mode))

(event OnComponentBeginOverlap(DoorTriggerLeft)
  (params (OverlappedComponent :type Primitive%20Component%20Object%20Reference) (OtherActor :type Actor%20Object%20Reference) (OtherComp :type Primitive%20Component%20Object%20Reference) (OtherBodyIndex :type Integer) (bFromSweep :type Boolean) (SweepResult :type Hit%20Result%20Structure%20%28by%20ref%29))
  ;[0 0 0] Door transition triggers
  (bind _asbp_player_char (Utilities|Casting|CastToBP_PlayerChar OtherActor))
  (Variables|/Game/Blueprints/BP_PlayerChar.BP_PlayerChar_C|SetIsMovingThroughDoor _asbp_player_char true)
  (Variables|/Game/Blueprints/BP_PlayerChar.BP_PlayerChar_C|SetNewSpawnLocation _asbp_player_char (Transformation|GetWorldLocation (Variables|Default|GetRightSpawnLocation)))
  (Variables|/Game/Blueprints/BP_PlayerChar.BP_PlayerChar_C|SetCurrentCam _asbp_player_char (Variables|Default|GetRightCamera))
  (bind _asbp_main_game_mode (Utilities|Casting|CastToBP_MainGameMode (Game|GetGameMode)))
  (Default|RoomTransition _asbp_main_game_mode))

(event EventBeginPlay
  ;[0 0 0] Get cameras
  (Utilities|FlowControl|Delay 0.0)
  (bind _asbp_camera (Utilities|Casting|CastToBP_Camera (Utilities|Array|Get(acopy) (Collision|GetOverlappingActors (Variables|Default|GetRightSpawnLocation) "/Game/Blueprints/BP_Camera.BP_Camera_C" :!class /Script/Engine.PrimitiveComponent))))
  (Variables|Default|SetRightCamera _asbp_camera)
  (bind _asbp_camera_2 (Utilities|Casting|CastToBP_Camera (Utilities|Array|Get(acopy) (Collision|GetOverlappingActors (Variables|Default|GetLeftSpawnLocation) "/Game/Blueprints/BP_Camera.BP_Camera_C" :!class /Script/Engine.PrimitiveComponent))))
  (Variables|Default|SetLeftCamera _asbp_camera_2))

(fn ConstructionScript)