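; Level 1 end scene actor that plays a short cutscene and brings up the level-end screen.
; On BeginPlay it disables player input, while Tick auto-walks the BP_PlayerChar along +X as long as its IsInCutscene flag is set.
; A delay chain clears that flag to stop the walk, adds the WB_Level1End widget, pauses the game, then switches to UI-only input with a visible cursor.
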(event Custom|MoveChar
  (bind _returnvalue (Game|Player|GetPlayerPawn 0))
  (if (Variables|/Game/Blueprints/Player/BP_PlayerChar.BP_PlayerChar_C|GetIsInCutscene (.AsBP%20Player%20Char (Utilities|Casting|CastToBP_PlayerChar _returnvalue)))
    (bind _asbp_player_char (Utilities|Casting|CastToBP_PlayerChar _returnvalue))
    (Pawn|Input|AddMovementInput _asbp_player_char "0.500000, 0, 0" 1.0 false)))

(event EventBeginPlay
  (bind _returnvalue (Game|Player|GetPlayerPawn 0))
  (bind _returnvalue_2 (Game|GetPlayerController 0))
  (Input|DisableInput _returnvalue _returnvalue_2)
  (Utilities|FlowControl|Delay 1.5)
  (Variables|/Game/Blueprints/Player/BP_PlayerChar.BP_PlayerChar_C|SetIsInCutscene (.AsBP%20Player%20Char (Utilities|Casting|CastToBP_PlayerChar _returnvalue)) false)
  (Utilities|FlowControl|Delay 2.0)
  (bind _returnvalue_3 (UserInterface|CreateWidget "/Game/UI/LevelOutros/WB_Level1End.WB_Level1End_C" _returnvalue_2))
  (UserInterface|Viewport|AddtoViewport _returnvalue_3 2)
  (Utilities|FlowControl|Delay 1.0)
  (Game|SetGamePaused true)
  (Utilities|FlowControl|Delay 4.75)
  (Input|SetInputModeUIOnly _returnvalue_2 0 "DoNotLock")
  (Variables|/Script/Engine.PlayerController|SetbShowMouseCursor _returnvalue_2 true))

(event EventTick
  (params (DeltaSeconds :type Float%20%28single-precision%29))
  (CallFunction|MoveChar))

(fn ConstructionScript)