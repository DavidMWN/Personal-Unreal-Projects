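; BP_Camera_Restricter is a placeable volume that confines the player's camera to an X/Z area, apparently for a side-view game.
; When BP_PlayerChar enters or leaves the trigger box, it activates or deactivates itself as a restricter on that player's CurrentCam.
; The construction script sizes both boxes from exposed variables, scaling the confines in 16:9 units.
; On BeginPlay it caches min/max limits from the confines bounds, inset by half a fixed 256x144 extent.
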(event OnComponentBeginOverlap(PlayerTriggerBox)
  (params (OverlappedComponent :type Primitive%20Component%20Object%20Reference) (OtherActor :type Actor%20Object%20Reference) (OtherComp :type Primitive%20Component%20Object%20Reference) (OtherBodyIndex :type Integer) (bFromSweep :type Boolean) (SweepResult :type Hit%20Result%20Structure%20%28by%20ref%29))
  (bind _asbp_player_char (Utilities|Casting|CastToBP_PlayerChar OtherActor))
  (Default|SetRestricterActive (Variables|/Game/Blueprints/Player/BP_PlayerChar.BP_PlayerChar_C|GetCurrentCam _asbp_player_char) self))

(event OnComponentEndOverlap(PlayerTriggerBox)
  (params (OverlappedComponent :type Primitive%20Component%20Object%20Reference) (OtherActor :type Actor%20Object%20Reference) (OtherComp :type Primitive%20Component%20Object%20Reference) (OtherBodyIndex :type Integer))
  (bind _asbp_player_char (Utilities|Casting|CastToBP_PlayerChar OtherActor))
  (Default|SetRestricterInactive (Variables|/Game/Blueprints/Player/BP_PlayerChar.BP_PlayerChar_C|GetCurrentCam _asbp_player_char) self))

(event EventBeginPlay
  (Utilities|GetConfinesBoxBounds))

(fn ConstructionScript
  (Transformation|SetRelativeTransform (Variables|Default|GetPlayerTriggerBox) (Variables|Trigger|GetPlayerTriggerTransform) false false)
  (Components|Box|SetBoxExtent (Variables|Default|GetPlayerTriggerBox) (Variables|Trigger|GetPlayerTriggerExtend) true)
  (Components|Box|SetBoxExtent (Variables|Default|GetCollisionConfinesBox) (Math|Vector|MakeVector (* (* (Variables|RoomSize|GetConfinerWidth) 8.0) 16.0) 1e+01 (* (* (Variables|RoomSize|GetConfinerHeight) 8.0) 9.0)) true))