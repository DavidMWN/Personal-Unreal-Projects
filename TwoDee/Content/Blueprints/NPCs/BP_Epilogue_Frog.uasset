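; Epilogue frog NPC that shows dialogue and drives the ending UI through overlaps on its trigger box.
; When the player enters, it clears their cutscene flag, reveals and initiates the frog text widget, then adds the epilogue widget after a delay.
; When the player leaves, it hides the text and, after a shorter delay, adds the cutscene fade-out widget and plays its animation.
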(event OnComponentBeginOverlap(Box)
  (params (OverlappedComponent :type Primitive%20Component%20Object%20Reference) (OtherActor :type Actor%20Object%20Reference) (OtherComp :type Primitive%20Component%20Object%20Reference) (OtherBodyIndex :type Integer) (bFromSweep :type Boolean) (SweepResult :type Hit%20Result%20Structure%20%28by%20ref%29))
  (bind _helptext (Variables|Default|GetHelpText))
  (bind _asbp_player_char (Utilities|Casting|CastToBP_PlayerChar OtherActor))
  (Variables|/Game/Blueprints/Player/BP_PlayerChar.BP_PlayerChar_C|SetIsInCutscene _asbp_player_char false)
  (Development|SetHiddeninGame _helptext false false)
  (Default|Initiate (.AsBP%20Frog%20Text%20Epilogue (Utilities|Casting|CastToBP_FrogText_Epilogue (UserInterface|GetUserWidgetObject _helptext))))
  (Utilities|FlowControl|Delay 5.0)
  (bind _returnvalue (UserInterface|CreateWidget "/Game/UI/LevelIntros/WB_Epilogue.WB_Epilogue_C" (Game|GetPlayerController 0)))
  (UserInterface|Viewport|AddtoViewport _returnvalue 0))

(event OnComponentEndOverlap(Box)
  (params (OverlappedComponent :type Primitive%20Component%20Object%20Reference) (OtherActor :type Actor%20Object%20Reference) (OtherComp :type Primitive%20Component%20Object%20Reference) (OtherBodyIndex :type Integer))
  (Utilities|Casting|CastToBP_PlayerChar OtherActor)
  (Development|SetHiddeninGame (Variables|Default|GetHelpText) true false)
  (Utilities|FlowControl|Delay 3.0)
  (bind _returnvalue (UserInterface|CreateWidget "/Game/UI/LevelIntros/WB_CutsceneFadeOut.WB_CutsceneFadeOut_C" (Game|GetPlayerController 0)))
  (UserInterface|Viewport|AddtoViewport _returnvalue 0)
  (UserInterface|Animation|PlayAnimation _returnvalue (Variables|/Game/UI/LevelIntros/WB_CutsceneFadeOut.WB_CutsceneFadeOut_C|GetFadeOut _returnvalue) 0.0 1 "Forward" 1.0 false))

(fn ConstructionScript)