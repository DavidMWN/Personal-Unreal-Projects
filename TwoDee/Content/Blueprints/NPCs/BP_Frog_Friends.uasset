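; Friendly-named frog NPC that wanders by hopping back and forth along the X axis with flipbook animation.
; Tick calls two events whose pending Delays act as timers.
; MovementTimer waits a random few seconds, flips direction after a small random hop count, then sets IsHopping.
; While that flag is set, HopForward faces the sprite, jumps and adds movement input, returning to idle after a short delay.
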(event Custom|MovementTimer
  (Utilities|FlowControl|Delay (Math|Random|RandomFloatinRange 2.0 4.0))
  (if (>= (Variables|Default|GetHopCount) (Math|Random|RandomInteger 2))
    (Variables|Default|SetIsMovingRight (not (Variables|Default|GetIsMovingRight)))
    (Variables|Default|SetHopCount 0)
    (else
      (Math|Integer|IncrementInt (Variables|Default|GetHopCount)
        (:%20%20
          _))))
  (Variables|Default|SetIsHopping true))

(event Custom|HopForward
  (if (Variables|Default|GetIsHopping)
    (Transformation|SetRelativeRotation (Variables|Default|GetSprite) (Math|Rotator|MakeRotator 0.0 0.0 (Math|Float|SelectFloat 0.0 1.8e+02 (Variables|Default|GetIsMovingRight))) false false)
    (Sprite|SetFlipbook (Variables|Default|GetSprite) "/Game/SunnyLandAssets/sprites/frog/jump/frog-jump.frog-jump")
    (Character|Jump)
    (Pawn|Input|AddMovementInput (Math|Vector|SelectVector "-1.000000, 0, 0" "1.000000, 0, 0" (Variables|Default|GetIsMovingRight)) 1.0 false)
    (Utilities|FlowControl|Delay 0.4)
    (Sprite|SetFlipbook (Variables|Default|GetSprite) "/Game/SunnyLandAssets/sprites/frog/idle/frog-idle1.frog-idle1")
    (Variables|Default|SetIsHopping false)))

(event EventTick
  (params (DeltaSeconds :type Float%20%28single-precision%29))
  (CallFunction|MovementTimer)
  (CallFunction|HopForward))

(fn ConstructionScript)