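; Flying eagle enemy that patrols back and forth while bobbing up and down.
; Tick re-triggers two Delay-based timers that toggle horizontal and vertical direction flags, with the horizontal flag flipping less often.
; While alive, those flags set the sprite's yaw and drive movement input along X and Z.
; Once dead, input stops and high flying braking deceleration keeps the death animation from drifting along the flight path.
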(event Custom|ControlRotation
  ;[0 0 0] Patrol Movement
  (if (Variables|Default|GetIsDead)
    ;;[0 0 0] Needed this to stop death anim from continuing along flight path.
    (Variables|/Script/Engine.CharacterMovementComponent|SetBrakingDecelerationFlying (Variables|Character|GetCharacterMovement) 1e+03)
    (else
      (Transformation|SetRelativeRotation (Variables|Default|GetSprite) (Math|Rotator|MakeRotator 0.0 0.0 (Math|Float|SelectFloat 0.0 1.8e+02 (Variables|Default|GetIsMovingRight))) false false)
      (Pawn|Input|AddMovementInput (Math|Vector|MakeVector (.x (Math|Vector|SelectVector "-1.000000, 0,0.000000" "1.000000, 0,0.000000" (Variables|Default|GetIsMovingRight))) 0.0 (.z (Math|Vector|SelectVector "0.000000, 0,-1.000000" "0.000000, 0,1.000000" (Variables|Default|GetIsMovingDown)))) 1.0 false))))

(event Custom|MovementTimer
  ;[0 0 0] Patrol Movement
  (Utilities|FlowControl|Delay 2.0)
  (Variables|Default|SetIsMovingRight (not (Variables|Default|GetIsMovingRight))))

(event Custom|VerticalTimer
  ;[0 0 0] Patrol Movement
  (Utilities|FlowControl|Delay 1.0)
  (Variables|Default|SetIsMovingDown (not (Variables|Default|GetIsMovingDown))))

(event EventTick
  (params (DeltaSeconds :type Float%20%28single-precision%29))
  (CallFunction|MovementTimer)
  (CallFunction|VerticalTimer)
  (CallFunction|ControlRotation))

(fn ConstructionScript
  (|CallParentFunction))