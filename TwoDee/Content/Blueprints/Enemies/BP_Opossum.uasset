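; BP_Opossum is a patrolling 2D enemy that damages the player on contact.
; Tick drives a two-second Delay that flips the movement direction, then feeds movement input along X and yaws the Paper2D sprite to match.
; Overlapping its Box takes one health from BP_PlayerChar.
; Death stops the patrol, disables collision, plays the death flipbook and destroys the actor after a short delay.
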(event OnComponentBeginOverlap(Box)
  (params (OverlappedComponent :type Primitive%20Component%20Object%20Reference) (OtherActor :type Actor%20Object%20Reference) (OtherComp :type Primitive%20Component%20Object%20Reference) (OtherBodyIndex :type Integer) (bFromSweep :type Boolean) (SweepResult :type Hit%20Result%20Structure%20%28by%20ref%29))
  ;[0 0 0] Contact with Player (cause damage)
  (bind _asbp_player_char (Utilities|Casting|CastToBP_PlayerChar OtherActor))
  (Default|ChangeHealth _asbp_player_char -1))

(event Custom|ControlRotation
  ;[0 0 0] Patrol Movement
  (if (not (Variables|Default|GetIsDead))
    (Transformation|SetRelativeRotation (Variables|Default|GetSprite) (Math|Rotator|MakeRotator 0.0 0.0 (Math|Float|SelectFloat 0.0 1.8e+02 (Variables|Default|GetIsMovingRight))) false false)
    (Pawn|Input|AddMovementInput (Math|Vector|SelectVector "-1.000000, 0, 0" "1.000000, 0, 0" (Variables|Default|GetIsMovingRight)) 1.0 false)))

(event Custom|MovementTimer
  ;[0 0 0] Patrol Movement
  (Utilities|FlowControl|Delay 2.0)
  (Variables|Default|SetIsMovingRight (not (Variables|Default|GetIsMovingRight))))

(event Custom|Death
  ;[0 0 0] Death event
  (Variables|Default|SetIsDead true)
  (Sprite|SetFlipbook (Variables|Default|GetSprite) "/Game/SunnyLandAssets/sprites/enemy-death/enemy-death.enemy-death")
  (Collision|SetCollisionEnabled (Variables|Default|GetBox) "NoCollision")
  (Utilities|FlowControl|Delay 0.8)
  (Actor|DestroyActor))

(event EventTick
  (params (DeltaSeconds :type Float%20%28single-precision%29))
  (CallFunction|MovementTimer)
  (CallFunction|ControlRotation))

(fn ConstructionScript)