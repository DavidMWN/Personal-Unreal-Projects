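; Flying eagle boss for a 2D level, with its own health bar, that removes an invisible wall on death.
; Tick drives flight between left and right points, randomly swooping through a lower point with limits on repeats and gaps.
; A random Delay re-arms volleys of three throwing stars.
; Player star hits update the bar and trigger brief invincibility with a material flash, supplementing BP_Enemies damage logic.
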(event OnComponentBeginOverlap(Box)
  (params (OverlappedComponent :type Primitive%20Component%20Object%20Reference) (OtherActor :type Actor%20Object%20Reference) (OtherComp :type Primitive%20Component%20Object%20Reference) (OtherBodyIndex :type Integer) (bFromSweep :type Boolean) (SweepResult :type Hit%20Result%20Structure%20%28by%20ref%29))
  ;[0 0 0] Checks if player has damaged boss
  (Utilities|Casting|CastToBP_ThrowingStar OtherActor)
  (CallFunction|Damaged))

(event Custom|Throw
  ;[0 0 0] Throw projectile action
  (Audio|PlaySound2D "/Game/Sounds/AABossThrow.AABossThrow" 1.0 1.0 0.0 0 0)
  (Game|SpawnActorfromClass "/Game/Blueprints/Enemies/BP_BossThrowingStar.BP_BossThrowingStar_C" (Transformation|GetWorldTransform (Variables|Default|GetSpawnProjectile1)) "Undefined" 0 0)
  (Game|SpawnActorfromClass "/Game/Blueprints/Enemies/BP_BossThrowingStar.BP_BossThrowingStar_C" (Transformation|GetWorldTransform (Variables|Default|GetSpawnProjectile2)) "Undefined" 0 0)
  (Game|SpawnActorfromClass "/Game/Blueprints/Enemies/BP_BossThrowingStar.BP_BossThrowingStar_C" (Transformation|GetWorldTransform (Variables|Default|GetSpawnProjectile3)) "Undefined" 0 0))

(event Custom|Damaged
  ;[0 0 0] Actions when boss has taken damage. This is in addition to the Damaged Event defined in BP_Enemies.
  (if (not (Variables|Default|GetIsInvincible))
    (Audio|PlaySound2D "/Game/Sounds/AAEnemyDeath.AAEnemyDeath" 1.0 1.0 0.0 0 0)
    ;;[0 0 0] Set temp invincibility to stop player spamming boss to death
    (Variables|Default|SetIsInvincible true)
    ;;[0 0 0] Reduce health bar
    (Default|UpdateBossHealthBar (Variables|Default|GetHealthBarRef) (Math|Conversions|ToFloat(Integer) (Variables|Default|GetHealth)) (Math|Conversions|ToFloat(Integer) (Variables|Default|GetMaxHealth)))
    ;;[0 0 0] Boss changes to lighter color to indicate damage has been taken and is in invicible state
    (Rendering|Material|SetMaterial (Variables|Default|GetSprite) 0 "/Game/Materials/BossDmgSpriteMaterial.BossDmgSpriteMaterial")
    (Utilities|FlowControl|Delay 0.7)
    (Rendering|Material|SetMaterial (Variables|Default|GetSprite) 0 "/Paper2D/MaskedUnlitSpriteMaterial.MaskedUnlitSpriteMaterial")
    ;;[0 0 0] If Boss is dead, removes the health bar widget, otherwise removes Invincible status so player can damage again.
    (if (Variables|Default|GetIsDead)
      (Widget|RemovefromParent (Variables|Default|GetHealthBarRef))
      (Actor|DestroyActor (Variables|Default|GetInvisWall))
      (else
        (Variables|Default|SetIsInvincible false)))))

(event Custom|ThrowTimer
  ;[0 0 0] Timer to control rate of throwing
  (Utilities|FlowControl|Delay (Math|Random|RandomFloatinRange 1.75 2.5))
  (Variables|Default|SetCanThrow true))

(event Custom|DoAction
  ;[0 0 0] Main action controller
  (if (not (Variables|Default|GetIsDead))
    (if (Variables|Default|GetCanThrow)
      (CallFunction|Throw)
      (Variables|Default|SetCanThrow false))))

(event Custom|ControlRotation
  ;[0 0 0] Flips sprite left/right as appropriate
  (Transformation|SetRelativeRotation (Variables|Default|GetSprite) (Math|Rotator|MakeRotator 0.0 0.0 (Math|Float|SelectFloat 1.8e+02 0.0 (Variables|Default|GetIsMovingRight))) false false))

(event Custom|Movement
  (params (DeltaSeconds :type Float%20%28double-precision%29))
  (bind _self self)
  (bind _self_2 self)
  (bind _self_3 self)
  (bind _pointright (Variables|Default|GetPointRight))
  (bind _charactermovement (Variables|Character|GetCharacterMovement))
  (bind _pointleft (Variables|Default|GetPointLeft))
  (bind _pointswoop (Variables|Default|GetPointSwoop))
  (bind _returnvalue (Transformation|GetActorLocation _self))
  (bind _returnvalue_2 (Transformation|GetActorLocation _pointswoop))
  (bind _returnvalue_3 (Transformation|GetActorLocation _pointright))
  (bind _returnvalue_4 (Transformation|GetActorLocation _self_2))
  (bind _returnvalue_5 (Transformation|GetActorLocation _pointleft))
  (bind _returnvalue_6 (Transformation|GetActorLocation _self_3))
  (bind _maxflyspeed (Variables|/Script/Engine.CharacterMovementComponent|GetMaxFlySpeed _charactermovement))
  (bind _returnvalue_7 (- (Math|Vector|MakeVector (.x _returnvalue_2) 0.0 (.z _returnvalue_2)) (Math|Vector|MakeVector (.x _returnvalue) 0.0 (.z _returnvalue))))
  (bind _returnvalue_8 (- (Math|Vector|MakeVector (.x _returnvalue_3) 0.0 (.z _returnvalue_3)) (Math|Vector|MakeVector (.x _returnvalue_4) 0.0 (.z _returnvalue_4))))
  (bind _returnvalue_9 (* DeltaSeconds _maxflyspeed))
  (bind _returnvalue_10 (- (Math|Vector|MakeVector (.x _returnvalue_5) 0.0 (.z _returnvalue_5)) (Math|Vector|MakeVector (.x _returnvalue_6) 0.0 (.z _returnvalue_6))))
  ;[0.005208 0.005208 0.005208] Controls the Eagle Boss' movement
  (if (Variables|Default|GetIsDead)
    (Variables|/Script/Engine.CharacterMovementComponent|SetBrakingDecelerationFlying (Variables|Character|GetCharacterMovement) 1e+03)
    (elif (Variables|Default|GetIsSwooping)
      ;;[0 0 0] Movement to a third point in between and below the other two points (a swoop)
      (Variables|Default|SetCountNoSwoop 0)
      (Pawn|Input|AddMovementInput (Math|Vector|MakeVector (.x _returnvalue_7) 0.0 (.z _returnvalue_7)) _returnvalue_9 false)
      ;;[0 0 0] Checks if swoop point has been reached, turns IsSwooping to False, does NOT flip IsMovingRight so boss will continue in X direction to the normal Left or Right point.
      (if (Utilities|Operators|EqualEqual (Math|Vector|MakeVector (.x _returnvalue_2) 0.0 (.z _returnvalue_2)) (Math|Vector|MakeVector (.x _returnvalue) 0.0 (.z _returnvalue)) 5.0)
        (Variables|Default|SetIsSwooping false))
      (elif (Variables|Default|GetIsMovingRight)
        ;;[0 0 0] Normal left/right movement between two points
        (Pawn|Input|AddMovementInput (Math|Vector|MakeVector (.x _returnvalue_8) 0.0 (.z _returnvalue_8)) _returnvalue_9 false)
        ;;[0 0 0] Checks if point has been reached, flips IsMovingRight value to turn around
        (if (Utilities|Operators|EqualEqual (Math|Vector|MakeVector (.x _returnvalue_3) 0.0 (.z _returnvalue_3)) (Math|Vector|MakeVector (.x _returnvalue_4) 0.0 (.z _returnvalue_4)) 5.0)
          (Variables|Default|SetIsMovingRight false)
          ;;[0 0 0] Random value to check if boss should Swoop or not.
          (if (> (Math|Random|RandomFloatinRange 0.0 1e+01) 5.0) :!label _label
            ;;[0 0 0] Prevents boss from Swooping twice in a row, or from not swooping for more than value of MaxNoSwoop.
            (if (== (Variables|Default|GetCountNoSwoop) 0)
              (Math|Integer|IncrementInt (Variables|Default|GetCountNoSwoop))
              (else
                (Variables|Default|SetIsSwooping true :!label _label_2)))
            (elif (== (Variables|Default|GetCountNoSwoop) (Variables|Default|GetMaxNoSwoop))
              (goto _label_2)
              (else
                (Math|Integer|IncrementInt (Variables|Default|GetCountNoSwoop))))))
        (else
          (Pawn|Input|AddMovementInput (Math|Vector|MakeVector (.x _returnvalue_10) 0.0 (.z _returnvalue_10)) _returnvalue_9 false)
          (if (Utilities|Operators|EqualEqual (Math|Vector|MakeVector (.x _returnvalue_5) 0.0 (.z _returnvalue_5)) (Math|Vector|MakeVector (.x _returnvalue_6) 0.0 (.z _returnvalue_6)) 5.0)
            (Variables|Default|SetIsMovingRight true)
            (goto _label)))))))

(event EventBeginPlay
  ;[0 0 0] Adds boss health bar to player screen
  (bind _returnvalue (UserInterface|CreateWidget "/Game/UI/PlayerHUD/WB_BossHealth.WB_BossHealth_C"))
  (UserInterface|Viewport|AddtoViewport _returnvalue 0)
  (Variables|Default|SetHealthBarRef _returnvalue))

(event EventTick
  (params (DeltaSeconds :type Float%20%28single-precision%29))
  (CallFunction|Movement DeltaSeconds)
  (CallFunction|ThrowTimer)
  (CallFunction|ControlRotation)
  (CallFunction|DoAction))

(fn ConstructionScript
  (|CallParentFunction))