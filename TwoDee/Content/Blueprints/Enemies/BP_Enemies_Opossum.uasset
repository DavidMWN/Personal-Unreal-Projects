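; Opossum enemy Blueprint that patrols back and forth along the X axis until IsDead is set.
; Tick calls MovementTimer and ControlRotation every frame, relying on Delay ignoring retriggers to flip IsMovingRight about every two seconds.
; While alive, ControlRotation yaws the Sprite to face either way and feeds the matching direction into AddMovementInput.
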(event Custom|ControlRotation
  ;[0 0 0] Patrol Movement
  (if (not (Variables|Default|GetIsDead))
    (Transformation|SetRelativeRotation (Variables|Default|GetSprite) (Math|Rotator|MakeRotator 0.0 0.0 (Math|Float|SelectFloat 0.0 1.8e+02 (Variables|Default|GetIsMovingRight))) false false)
    (Pawn|Input|AddMovementInput (Math|Vector|SelectVector "-1.000000, 0, 0" "1.000000, 0, 0" (Variables|Default|GetIsMovingRight)) 1.0 false)))

(event Custom|MovementTimer
  ;[0 0 0] Patrol Movement
  (Utilities|FlowControl|Delay 2.0)
  (Variables|Default|SetIsMovingRight (not (Variables|Default|GetIsMovingRight))))

(event EventTick
  (params (DeltaSeconds :type Float%20%28single-precision%29))
  (CallFunction|MovementTimer)
  (CallFunction|ControlRotation))

(fn ConstructionScript
  (|CallParentFunction))