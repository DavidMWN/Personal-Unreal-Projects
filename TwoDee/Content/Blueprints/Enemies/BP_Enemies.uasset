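; BP_Enemies is a 2D flipbook enemy character that damages the player on contact and awards score when killed.
; Overlapping its Box takes one health from the player, while TakeDamage lowers its own Health unless invincible and triggers Death at zero.
; Death adds ScoreValue to the player, freezes movement, disables collision, plays sound and death flipbook, shows a points widget, then destroys the actor after a short delay.
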(event OnComponentBeginOverlap(Box)
  (params (OverlappedComponent :type Primitive%20Component%20Object%20Reference) (OtherActor :type Actor%20Object%20Reference) (OtherComp :type Primitive%20Component%20Object%20Reference) (OtherBodyIndex :type Integer) (bFromSweep :type Boolean) (SweepResult :type Hit%20Result%20Structure%20%28by%20ref%29))
  ;[0 0 0] Contact with Player (cause damage)
  (bind _asbp_player_char (Utilities|Casting|CastToBP_PlayerChar OtherActor))
  (Default|ChangeHealth _asbp_player_char -1))

(event Custom|TakeDamage
  (bind _health (Variables|Default|GetHealth))
  ;[0 0 0] Damaged Event
  (if (not (Variables|Default|GetIsInvincible))
    (Math|Integer|DecrementInt _health
      (:%20%20
        (if (== _health 0)
          (CallFunction|Death))))))

(event Custom|Death
  (bind _points (Variables|Default|GetPoints))
  (bind _charactermovement (Variables|Character|GetCharacterMovement))
  ;[0 0 0] Death event
  (Variables|Default|SetIsDead true)
  (bind _asbp_player_char (Utilities|Casting|CastToBP_PlayerChar (Game|Player|GetPlayerPawn 0)))
  (Default|IncreaseScore _asbp_player_char (Variables|Default|GetScoreValue))
  (Components|Movement|StopMovementImmediately _charactermovement)
  (Variables|/Script/Engine.CharacterMovementComponent|SetGravityScale _charactermovement 0.0)
  (Audio|PlaySound2D (Variables|Default|GetDeathSound) 1.0 1.0 0.0 0 0)
  (Sprite|SetFlipbook (Variables|Default|GetSprite) "/Game/SunnyLandAssets/sprites/enemy-death/enemy-death.enemy-death")
  (Development|SetHiddeninGame _points false false)
  (bind _aswb_points (Utilities|Casting|CastToWB_Points (UserInterface|GetUserWidgetObject _points)))
  (Default|ShowPoints _aswb_points (Variables|Default|GetScoreValue))
  (Collision|SetCollisionEnabled (Variables|Default|GetBox) "NoCollision")
  (Utilities|FlowControl|Delay 0.8)
  (Actor|DestroyActor))

(fn ConstructionScript)