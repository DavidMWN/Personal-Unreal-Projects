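; Boss enemy, extending the BP_Enemies damage logic, that jumps and throws BP_BossThrowingStar projectiles at random intervals.
; Tick runs Delay-based timers that set jump and throw flags, which DoAction consumes while the boss is alive.
; Overlaps from BP_ThrowingStar trigger Damaged, which updates an on-screen health bar and grants brief invincibility with a lighter sprite material.
; The health bar is created at BeginPlay and removed after death.
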(event OnComponentBeginOverlap(Box)
  (params (OverlappedComponent :type Primitive%20Component%20Object%20Reference) (OtherActor :type Actor%20Object%20Reference) (OtherComp :type Primitive%20Component%20Object%20Reference) (OtherBodyIndex :type Integer) (bFromSweep :type Boolean) (SweepResult :type Hit%20Result%20Structure%20%28by%20ref%29))
  ;[0 0 0] Checks if player has damaged boss
  (Utilities|Casting|CastToBP_ThrowingStar OtherActor)
  (CallFunction|Damaged))

(event Custom|Throw
  ;[0 0 0] Throw projectile action
  (Game|SpawnActorfromClass "/Game/Blueprints/Enemies/BP_BossThrowingStar.BP_BossThrowingStar_C" (Transformation|GetWorldTransform (Variables|Default|GetSpawnProjectile)) "Undefined" 0 0))

(event Custom|Damaged
  ;[0 0 0] Actions when boss has taken damage. This is in addition to the Damaged Event defined in BP_Enemies.
  ;;[0 0 0] Set temp invincibility to stop player spamming boss to death
  (Variables|Default|SetIsInvincible true)
  ;;[0 0 0] Reduce health bar
  (Default|UpdateBossHealthBar (Variables|Default|GetHealthBarRef) (Math|Conversions|ToFloat(Integer) (Variables|Default|GetHealth)) (Math|Conversions|ToFloat(Integer) (Variables|Default|GetMaxHealth)))
  ;;[0 0 0] Boss changes to lighter color to indicate damage has been taken and is in invicible state
  (Rendering|Material|SetMaterial (Variables|Default|GetSprite) 0 "/Game/Materials/BossDmgSpriteMaterial.BossDmgSpriteMaterial")
  (Utilities|FlowControl|Delay 0.7)
  (Rendering|Material|SetMaterial (Variables|Default|GetSprite) 0 "/Paper2D/MaskedUnlitSpriteMaterial.MaskedUnlitSpriteMaterial")
  ;;[0 0 0] If Boss is dead, removes the health bar widget, otherwise removes Invincible status so player can damage again.
  (if (Variables|Default|GetIsDead)
    (Widget|RemovefromParent (Variables|Default|GetHealthBarRef))
    (else
      (Variables|Default|SetIsInvincible false))))

(event Custom|JumpTimer
  ;[0 0 0] Timers to control rate of jumping and throwing
  (Utilities|FlowControl|Delay (Math|Random|RandomFloatinRange 2.0 3.0))
  (Variables|Default|SetCanJumpUp true))

(event Custom|ThrowTimer
  ;[0 0 0] Timers to control rate of jumping and throwing
  (Utilities|FlowControl|Delay (Math|Random|RandomFloatinRange 1.75 2.5))
  (Variables|Default|SetCanThrow true))

(event Custom|DoAction
  ;[0 0 0] Main action controller
  (if (not (Variables|Default|GetIsDead))
    (if (Variables|Default|GetCanThrow)
      (CallFunction|Throw)
      (Variables|Default|SetCanThrow false))
    (if (Variables|Default|GetCanJumpUp)
      (Character|Jump)
      (Variables|Default|SetCanJumpUp false))))

(event EventBeginPlay
  ;[0 0 0] Adds boss health bar to player screen
  (bind _returnvalue (UserInterface|CreateWidget "/Game/UI/PlayerHUD/WB_BossHealth.WB_BossHealth_C"))
  (UserInterface|Viewport|AddtoViewport _returnvalue 0)
  (Variables|Default|SetHealthBarRef _returnvalue))

(event EventTick
  (params (DeltaSeconds :type Float%20%28single-precision%29))
  (CallFunction|JumpTimer)
  (CallFunction|ThrowTimer)
  (CallFunction|DoAction))

(fn ConstructionScript
  (|CallParentFunction))